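; BP_SecretTunnel is a wall that opens into a tunnel owned by the player who activates it.
; ActivateTunnel applies a dissolve material, switches the box to overlap collision, hides the cube after a short delay, and calls ChangeOwner.
; ChangeOwner stores the player ID and tints the plane with that player's emissive color.
; Non-owning Char_FlashlightKid players overlapping the box hear a cue and are launched along the arrow's forward direction.
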(event OnComponentBeginOverlap(Box)
  (params (OverlappedComponent :type Primitive%20Component%20Object%20Reference) (OtherActor :type Actor%20Object%20Reference) (OtherComp :type Primitive%20Component%20Object%20Reference) (OtherBodyIndex :type Integer) (bFromSweep :type Boolean) (SweepResult :type Hit%20Result%20Structure%20%28by%20ref%29))
  (bind _aschar_flashlight_kid (Utilities|Casting|CastToChar_FlashlightKid OtherActor))
  (if (Actor|ActorHasTag OtherActor "Player")
    (if (not (== (Variables|/Game/Blueprints/Char_FlashlightKid.Char_FlashlightKid_C|GetPlayerInt _aschar_flashlight_kid) (Variables|Default|GetOwningPlayer)))
      (Audio|PlaySound2D "/Game/Sounds/PushbackCue.PushbackCue" 1.0 1.0 0.0 0 0)
      (Character|LaunchCharacter _aschar_flashlight_kid (* (Math|Vector|GetForwardVector (Transformation|GetWorldRotation (Variables|Default|GetArrow))) 4000) false false))))

(event Custom|ActivateTunnel
  (params (PlayerID :type Integer))
  (bind _cube (Variables|Default|GetCube))
  (Rendering|Material|SetMaterial _cube 0 "/Game/Character_Appearance_Dissolve/Materials/Mobile/WallDissolve.WallDissolve")
  (CallFunction|ChangeOwner PlayerID)
  (Collision|SetCollisionProfileName (Variables|Default|GetBox) "OverlapAllDynamic" true :!class /Script/Engine.PrimitiveComponent)
  (Utilities|FlowControl|Delay 0.5)
  (Rendering|ToggleVisibility _cube false))

(event Custom|ChangeOwner
  (params (PlayerID :type Integer))
  (bind _plane (Variables|Default|GetPlane))
  (bind _output_get (Variables|Default|SetOwningPlayer PlayerID))
  (switch int _output_get
    (:0
      (Rendering|Material|SetMaterial _plane 0 "/Game/Materials/Emissive_Cyan.Emissive_Cyan"))
    (:1
      (Rendering|Material|SetMaterial _plane 0 "/Game/Materials/Emissive_Magenta.Emissive_Magenta"))
    (:2
      (Rendering|Material|SetMaterial _plane 0 "/Game/Materials/Emissive_Yellow.Emissive_Yellow"))
    (:3
      (Rendering|Material|SetMaterial _plane 0 "/Game/Materials/Emissive_Lime.Emissive_Lime"))))

(fn ConstructionScript)