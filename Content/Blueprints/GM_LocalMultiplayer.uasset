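; Local multiplayer game mode that runs a timed match from drop-in lobby to endgame menu.
; BeginPlay creates four local controllers possessing ReadyPlayerOne pawns, opens the drop-in menu, starts music and sets the countdown from MapMinutes.
; RunMatchStartup spawns and possesses a Char_FlashlightKid per active player, destroys lobby pawns, adds the HUD and activates a shared camera.
; Tick decrements the countdown through a one-second Delay, then pauses and opens the endgame menu.
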(event Custom|RunMatchStartup
  (params (ActivePlayers :type Integer))
  (Variables|Default|SetActivePlayers ActivePlayers)
  (CallFunction|SpawnPlayers)
  (CallFunction|SpawnCamera)
  (bind _returnvalue (UserInterface|CreateWidget "/Game/Widgets/W_HUD.W_HUD_C"))
  (UserInterface|Viewport|AddtoViewport _returnvalue 0)
  (Widget|RemovefromParent (Variables|Default|GetDropInMenu))
  (Input|SetInputModeGameOnly (Game|GetPlayerController 0))
  (Game|Player|SetViewTargetwithBlend (Game|GetPlayerController 0) (CallFunction|GetCamera) 0.0 "VTBlend_Linear" 0.0 false)
  (Utilities|FlowControl|Delay 0.2)
  (bind _outactors (Actor|GetAllActorsOfClass "/Game/Blueprints/ReadyPlayerOne_PawnBP.ReadyPlayerOne_PawnBP_C"))
  (for _array_element _outactors
    (Actor|DestroyActor _array_element))
  (Default|ActivateCamera (CallFunction|GetCamera))
  (Variables|Default|SetMatchStarted true))

(event EventBeginPlay
  (CallFunction|SpawnControllers)
  (bind _output_get (Variables|Default|SetOwningPlayer (.AsController%20Local%20Multiplayer (Utilities|Casting|CastToController_LocalMultiplayer (Game|GetPlayerController 0)))))
  (bind _widget (Default|OpenDropinMenu _output_get))
  (Variables|Default|SetDropInMenu _widget)
  (Variables|Default|SetCountdown (Math|Timespan|MakeTimespan 0 0 (Variables|Default|GetMapMinutes) 0 0))
  (Audio|PlaySound2D "/Game/Music/Jam1_-_Childlike.Jam1_-_Childlike" 0.75 1.0 0.0 0 0))

(event EventTick
  (params (DeltaSeconds :type Float%20%28single-precision%29))
  (if (Variables|Default|GetMatchStarted)
    (if (> (Variables|Default|GetCountdown) (Math|Timespan|MakeTimespan 0 0 0 0 0))
      (Utilities|FlowControl|Delay 1.0)
      (Variables|Default|SetCountdown (Math|Timespan|MakeTimespan 0 0 (.minutes (Variables|Default|GetCountdown)) (- (.seconds (Variables|Default|GetCountdown)) 1)))
      (else
        (Utilities|FlowControl|DoOnce false
          (:Completed
            (Viewport|RemoveAllWidgets)
            (Game|SetGamePaused true)
            (Default|OpenEndgameMenu (Variables|Default|GetOwningPlayer))))))))

(fn ConstructionScript)

(fn SpawnPlayers
  ;[1 1 1] Spawn Character Actors and Possess
  (for _index (range 0 (- (Variables|Default|GetActivePlayers) 1))
    (bind _returnvalue (Game|SpawnActorfromClass "/Game/Blueprints/Char_FlashlightKid.Char_FlashlightKid_C" (Math|Transform|MakeTransform "0.000000, 0,9000.000000") "Undefined" 0 _index 0))
    (Pawn|Possess (Game|GetPlayerController _index) _returnvalue)))

(fn SpawnCamera
  (bind _outactors (Actor|GetAllActorsOfClass "/Game/Blueprints/BP_CameraSpawn.BP_CameraSpawn_C"))
  (for _array_element _outactors
    (Default|SpawnCamera _array_element)))

(fn SpawnControllers
  ;[1 1 1] Add Player Controllers per Number of Players
  (for _index (range 1 3)
    (Class|GameplayStatics|CreatePlayer _index))
  ;[1 1 1] Spawn Character Actors and Possess
  (for _index_2 (range 0 3)
    (bind _returnvalue (Game|SpawnActorfromClass "/Game/Blueprints/ReadyPlayerOne_PawnBP.ReadyPlayerOne_PawnBP_C" (Math|Transform|MakeTransform "0.000000, 0,9000.000000") "Undefined" 0 _index_2 0 0))
    (Pawn|Possess (Game|GetPlayerController _index_2) _returnvalue)))

(fn GetCamera
  (bind _outactors (Actor|GetAllActorsOfClass "/Game/Blueprints/BP_LocalCamera.BP_LocalCamera_C"))
  (return (Utilities|Array|Get(acopy) _outactors)))