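; Shared local-multiplayer camera that frames up to four player characters once the match has started.
; ActivateCamera caches the characters and start height, then enables Tick.
; Each tick snaps the actor to the players' average XY position, while the spring arm eases toward its Box component plus an X offset at fixed height.
; The largest pairwise player distance drives smoothed arm-length zoom with a minimum clamp; an orthographic-width zoom is left disconnected.
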(event Custom|GetLongestDistanceBetweenPlayers
  (bind _character_0 (Variables|Default|GetCharacter_0))
  (bind _character_1 (Variables|Default|GetCharacter_1))
  (bind _character_2 (Variables|Default|GetCharacter_2))
  (bind _character_3 (Variables|Default|GetCharacter_3))
  ;[1 1 1] Check Longest Distance Between Players
  (Variables|Default|SetMaxDistance (+ (.MaxValue (Math|Float|MaxOfFloatArray (Utilities|Array|MakeArray (Transformation|GetDistanceTo _character_0 _character_1) (Transformation|GetDistanceTo _character_0 _character_2) (Transformation|GetDistanceTo _character_0 _character_3) (Transformation|GetDistanceTo _character_1 _character_2) (Transformation|GetDistanceTo _character_1 _character_3) (Transformation|GetDistanceTo _character_2 _character_3)))) 1e+02)))

(event Custom|SetCameraMidpoint
  ;[1 1 1] Determine Midpoint Between All Players
  (bind _output_get (Variables|Default|SetCameraMidpoint (/ (+ (Transformation|GetActorLocation (Variables|Default|GetCharacter_0)) (Transformation|GetActorLocation (Variables|Default|GetCharacter_1)) (Transformation|GetActorLocation (Variables|Default|GetCharacter_2)) (Transformation|GetActorLocation (Variables|Default|GetCharacter_3))) (Variables|/Game/Blueprints/GM_LocalMultiplayer.GM_LocalMultiplayer_C|GetActivePlayers (.AsGM%20Local%20Multiplayer (Utilities|Casting|CastToGM_LocalMultiplayer (Game|GetGameMode)))))))
  (Transformation|SetActorLocation (Math|Vector|MakeVector (.X (Math|Vector|BreakVector _output_get)) (.Y (Math|Vector|BreakVector _output_get)) (.z (Variables|Default|GetCameraStartPosition))) false false))

(event Custom|CameraZoom
  (bind _springarm (Variables|Default|GetSpringArm))
  ;[1 1 1] Camera Zoom
  (Variables|/Script/Engine.SpringArmComponent|SetTargetArmLength _springarm (Math|Interpolation|FInterpTo (Variables|/Script/Engine.SpringArmComponent|GetTargetArmLength _springarm) (Math|Float|Clamp(Float) (Variables|Default|GetMaxDistance) 9e+02 1.024e+12) (Variables|Default|GetDeltaSecondsTick) 1.5)))

(event Custom|SetCameraPosition
  (bind _box (Variables|Default|GetBox))
  (bind _deltasecondstick (Variables|Default|GetDeltaSecondsTick))
  (bind _returnvalue (Transformation|GetWorldLocation _box))
  ;[1 1 1] Set Camera Position
  (bind _output_get (Variables|Default|SetCameraYPosition (Math|Interpolation|FInterpTo (Variables|Default|GetCameraYPosition) (.y _returnvalue) _deltasecondstick 1.0)))
  (bind _output_get_2 (Variables|Default|SetCameraXPosition (Math|Interpolation|FInterpTo (Variables|Default|GetCameraXPosition) (+ (.x _returnvalue) (Variables|Default|GetXOffset)) _deltasecondstick 1.0)))
  (Transformation|SetWorldLocation (Variables|Default|GetSpringArm) (Math|Vector|MakeVector _output_get_2 _output_get (.z (Variables|Default|GetCameraStartPosition))) false false))

(event Custom|ActivateCamera
  (bind _returnvalue (Game|GetPlayerCharacter 1))
  (bind _returnvalue_2 (Game|GetPlayerCharacter 3))
  (bind _returnvalue_3 (Game|GetPlayerCharacter 0))
  (bind _returnvalue_4 (Game|GetPlayerCharacter 2))
  (bind _springarm (Variables|Default|GetSpringArm))
  (bind _returnvalue_5 (Transformation|GetWorldLocation _springarm))
  (Utilities|FlowControl|Sequence
    (:then_0
      (Utilities|FlowControl|Delay 0.01)
      (Utilities|IsValid _returnvalue_3
        (:Is%20Valid
          (Variables|Default|SetCharacter_0 _returnvalue_3)
          (Utilities|IsValid _returnvalue
            (:Is%20Valid
              (Variables|Default|SetCharacter_1 _returnvalue)
              (Utilities|IsValid _returnvalue_4
                (:Is%20Valid
                  (Variables|Default|SetCharacter_2 _returnvalue_4)
                  (Utilities|IsValid _returnvalue_2
                    (:Is%20Valid
                      (Variables|Default|SetCharacter_3 _returnvalue_2))
                    (:Is%20Not%20Valid
                      _)))
                (:Is%20Not%20Valid
                  _)))
            (:Is%20Not%20Valid
              _)))
        (:Is%20Not%20Valid
          _))
      (Actor|Tick|SetActorTickEnabled true))
    (:then_1
      (Variables|Default|SetCameraXPosition (.x _returnvalue_5))
      (Variables|Default|SetCameraYPosition (.y _returnvalue_5))
      (Variables|Default|SetCameraStartPosition (Math|Vector|MakeVector 0.0 0.0 (.z (Transformation|GetActorLocation))))
      (Utilities|FlowControl|Delay 0.1))))

(event EventTick
  (params (DeltaSeconds :type Float%20%28single-precision%29))
  (if (Variables|/Game/Blueprints/GM_LocalMultiplayer.GM_LocalMultiplayer_C|GetMatchStarted (.AsGM%20Local%20Multiplayer (Utilities|Casting|CastToGM_LocalMultiplayer (Game|GetGameMode))))
    (Variables|Default|SetDeltaSecondsTick DeltaSeconds)
    (CallFunction|GetLongestDistanceBetweenPlayers)
    (CallFunction|SetCameraMidpoint)
    (CallFunction|CameraZoom)
    (CallFunction|SetCameraPosition)))

(fn ConstructionScript)