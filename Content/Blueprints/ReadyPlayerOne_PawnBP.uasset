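; ReadyPlayerOne_PawnBP is a pawn that lets a local player join through the drop-in menu.
; The first DropIn press, gated by DoOnce, switches on the controller ID to activate one of four window templates in the DropInMenu held by GM_LocalMultiplayer.
; Each branch then increments the menu's active player count.
; Disconnected nodes for storing and printing the controller ID never run.
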(event Input|ActionEvents|InputActionDropIn
  (params (Key :type Key%20Structure))
  (:Pressed
    (Utilities|FlowControl|DoOnce false
      (:Completed
        (bind _asgm_local_multiplayer (Utilities|Casting|CastToGM_LocalMultiplayer (Game|GetGameMode)))
        (switch int (Variables|Default|GetPlayerControllerID)
          (:0
            (Variables|/Game/Widgets/WT_WindowTemplate.WT_WindowTemplate_C|SetActivated (Variables|/Game/Widgets/W_DropIn.W_DropIn_C|GetWindowTemplate_0 (Variables|/Game/Blueprints/GM_LocalMultiplayer.GM_LocalMultiplayer_C|GetDropInMenu _asgm_local_multiplayer)) true))
          (:1
            (Variables|/Game/Widgets/WT_WindowTemplate.WT_WindowTemplate_C|SetActivated (Variables|/Game/Widgets/W_DropIn.W_DropIn_C|GetWindowTemplate_1 (Variables|/Game/Blueprints/GM_LocalMultiplayer.GM_LocalMultiplayer_C|GetDropInMenu _asgm_local_multiplayer)) true))
          (:2
            (Variables|/Game/Widgets/WT_WindowTemplate.WT_WindowTemplate_C|SetActivated (Variables|/Game/Widgets/W_DropIn.W_DropIn_C|GetWindowTemplate_2 (Variables|/Game/Blueprints/GM_LocalMultiplayer.GM_LocalMultiplayer_C|GetDropInMenu _asgm_local_multiplayer)) true))
          (:3
            (Variables|/Game/Widgets/WT_WindowTemplate.WT_WindowTemplate_C|SetActivated (Variables|/Game/Widgets/W_DropIn.W_DropIn_C|GetWindowTemplate_3 (Variables|/Game/Blueprints/GM_LocalMultiplayer.GM_LocalMultiplayer_C|GetDropInMenu _asgm_local_multiplayer)) true)))
        (bind _result (Math|Integer|IncrementInt (Variables|/Game/Widgets/W_DropIn.W_DropIn_C|GetActivePlayers (Variables|/Game/Blueprints/GM_LocalMultiplayer.GM_LocalMultiplayer_C|GetDropInMenu _asgm_local_multiplayer)))
          (:%20%20
            (Variables|/Game/Widgets/W_DropIn.W_DropIn_C|SetActivePlayers (Variables|/Game/Blueprints/GM_LocalMultiplayer.GM_LocalMultiplayer_C|GetDropInMenu _asgm_local_multiplayer) _result)))))))

(fn ConstructionScript)